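; BP_PlayerTank is the player's tank Blueprint, and its graphs only handle team coloring.
; On BeginPlay it calls SetTeamColor for the base and turret meshes, passing TeamColor and a shared material parameter name.
; The same calls sit unconnected in the Construction Script, so the color is applied only at runtime.
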(event `self.ReceiveBeginPlay`
  (bind _teamcolormaterialparamname (`self.TeamColorMaterialParamName`))
  (bind _teamcolor (`self.TeamColor`))
  (`self.SetTeamColor` _teamcolormaterialparamname _teamcolor (`self.BaseMesh`))
  (`self.SetTeamColor` _teamcolormaterialparamname _teamcolor (`self.TurretMesh`)))

(event `self.ReceiveTick`
  (params (DeltaSeconds :type "Float (single-precision)")))

(fn `UserConstructionScript`
  (locals (NewLocalVar :type "StaticMeshComponent Object Reference")))